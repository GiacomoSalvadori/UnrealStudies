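; Playable third-person shooter character that adds feedback, throw aiming and death handling on top of inherited aim and weapon events.
; Trace-line shots trigger camera shake, weapon sound, muzzle flash and a noise event; reloads play a montage before EndReload.
; While arc-aiming, Tick destroys and respawns indicator actors along a predicted projectile path; stopping aim clears them.
; BeginPlay moves the audio listener to the mesh, and zero health opens MapTest after a delay.
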(event Custom|OnHealtToZero_Event_0
  (Utilities|FlowControl|Delay 3.0)
  (Game|OpenLevel(byName) "MapTest"))

(event Custom|OnCharacterAimNoise
  (bind _weaponmesh (Variables|Default|GetWeaponMesh))
  (bind _returnvalue (Transformation|GetWorldLocation _weaponmesh))
  (Class|PlayerCameraManager|PlayCameraShake (Game|GetPlayerCameraManager 0) "/Game/TPS/BP_CameraShake.BP_CameraShake_C" 1.0 "World" "0, 0, 0")
  (bind _returnvalue_2 (Class|TPThirdPersonCharacter|RetrieveActiveWeapon))
  (Audio|PlaySoundatLocation (.soundefx _returnvalue_2) _returnvalue "0, 0, 0" 1.0 1.0 0.0 0 0 0)
  (Class|AISenseHearing|ReportNoiseEvent _returnvalue 1.0 self 0.0 "None")
  (Effects|SpawnEmitteratLocation "/Game/EFX/P_BackPack_MuzzleFlash.P_BackPack_MuzzleFlash" (+ _returnvalue (* (Math|Vector|GetForwardVector _weaponmesh) 65.0)) (Transformation|GetWorldRotation (Variables|Character|GetMesh)) "0.100000,0.100000,0.100000"))

(event Custom|OnCharacterStopAim_Event_0
  (CallFunction|DeleteDrawIndicator))

(event Custom|OnCharacterStartReload_Event_0
  (Animation|Montage|PlayMontage (Variables|Character|GetMesh) "/Game/AnimStarterPack/Reload_Rifle_Hip_Montage.Reload_Rifle_Hip_Montage"
    (:OnCompleted
      (Class|TPThirdPersonCharacter|EndReload))))

(event EventTick
  (params (DeltaSeconds :type Float%20%28single-precision%29))
  (bind _returnvalue (Class|TPThirdPersonCharacter|IsAimingwithArch))
  (if _returnvalue
    (CallFunction|DrawThrowIndicator)))

(event EventBeginPlay
  (bind _mesh (Variables|Character|GetMesh))
  (EventDispatchers|AssignOnCharacterStartReload (delegate Custom|OnCharacterStartReload_Event_0))
  (EventDispatchers|BindEventtoOnCharacterTraceLine (delegate Custom|OnCharacterAimNoise))
  (EventDispatchers|AssignOnCharacterStopAim (delegate Custom|OnCharacterStopAim_Event_0))
  (Class|PlayerController|SetAudioListenerOverride (Game|GetPlayerController 0) _mesh (Transformation|GetWorldLocation _mesh) "0, 0, 0")
  (EventDispatchers|AssignOnHealttoZero (Variables|Default|GetHealthComponent) (delegate Custom|OnHealtToZero_Event_0)))

(fn ConstructionScript)

(fn DrawThrowIndicator
  (CallFunction|DeleteDrawIndicator)
  (bind _astp_third_person_character (Utilities|Casting|CastToTP_ThirdPersonCharacter (Game|GetPlayerCharacter 0)))
  (bind _returnvalue (Class|TPThirdPersonCharacter|PredictThrowablePath _astp_third_person_character))
  (bind _outpathpositions (Class|GameplayStatics|BlueprintPredictProjectilePathbyTraceChannel (Transformation|GetWorldLocation (Variables|/Script/UnrealStudies.TP_ThirdPersonCharacter|GetFollowCamera _astp_third_person_character)) _returnvalue true 1.0 "ECC_WorldDynamic" false (Utilities|Array|MakeArray self) "None"))
  (for (_array_element _array_index) _outpathpositions
    (if (and (> _array_index 9) (== (Math|Integer|%(Integer) _array_index 2) 0))
      (Game|SpawnActorfromClass "/Game/TPS/BP_ThrowIndicator.BP_ThrowIndicator_C" (Math|Transform|MakeTransform _array_element) "Undefined" 0 0))))

(fn DeleteDrawIndicator
  (bind _outactors (Actor|GetAllActorsOfClass "/Game/TPS/BP_ThrowIndicator.BP_ThrowIndicator_C"))
  (for _array_element _outactors
    (Actor|DestroyActor _array_element)))