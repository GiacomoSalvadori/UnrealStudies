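; BP_throwable is a timed throwable actor for the TPS game that bursts into an explosion effect, like a grenade.
; On BeginPlay it applies the WeaponMesh to its mesh and launches it by setting the physics linear velocity to Toss.
; Tick accumulates elapsed time until TimeToDestroy, then spawns the explosion particles at the mesh location and destroys the actor.
; The explosion is visual only, with no damage logic here.
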(event EventBeginPlay
  (bind _mesh (Variables|Default|GetMesh))
  (Components|StaticMesh|SetStaticMesh _mesh (Variables|Default|GetWeaponMesh))
  (Physics|SetPhysicsLinearVelocity _mesh (Variables|Default|GetToss) false "None"))

(event EventTick
  (params (DeltaSeconds :type Float%20%28single-precision%29))
  (bind _output_get (Variables|Default|SetElapsedTime (+ DeltaSeconds (Variables|Default|GetElapsedTime))))
  (if (>= _output_get (Variables|Default|GetTimeToDestroy))
    (Effects|SpawnEmitteratLocation "/Game/StarterContent/Particles/P_Explosion.P_Explosion" (Transformation|GetWorldLocation (Variables|Default|GetMesh)))
    (Actor|DestroyActor)))

(fn ConstructionScript)