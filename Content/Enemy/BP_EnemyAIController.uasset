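; Enemy AI controller that runs the BP_Enemy_BT behavior tree on BeginPlay and feeds it perception results.
; On perception updates, it loops through each updated actor's last sensed stimuli and treats index 0 as sight.
; ManageSight writes that stimulus's success flag to the SeePlayer blackboard key, without checking that the actor is the player, and prints the blackboard's name.
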(event OnPerceptionUpdated(PerceptionComponent)
  (params (UpdatedActors :type Array%20of%20Actor%20Object%20References))
  (for _array_element UpdatedActors
    (bind _info (Class|AIPerceptionComponent|GetActorsPerception (Class|AIController|GetAIPerceptionComponent) _array_element))
    (for (_array_element_2 _array_index) (.lastsensedstimuli _info)
      (Variables|Default|SetLocal%20Sense _array_element_2)
      (switch int _array_index
        (:0
          (CallFunction|ManageSight (Variables|Default|GetLocal%20Sense)))))))

(event EventBeginPlay
  (AI|RunBehaviorTree "/Game/Enemy/BP_Enemy_BT.BP_Enemy_BT"))

(fn ConstructionScript)

(fn ManageSight
  (params (Sense :type AI%20Stimulus%20Structure))
  (bind _returnvalue (AI|GetBlackboard 0))
  (Development|PrintString (Utilities|GetDisplayName _returnvalue))
  (AI|Components|Blackboard|SetValueasBool _returnvalue (Utilities|Name|MakeLiteralName "SeePlayer") (.bsuccessfullysensed Sense)))