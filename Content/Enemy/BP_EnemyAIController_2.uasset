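; BP_EnemyAIController_2 is an enemy AI controller with a perception component, but its perception update event currently does nothing.
; A disconnected chain loops over updated actors and their last sensed stimuli, treating the first index as sight and the second as damage.
; It would pass sight to ManageSight, which writes the SeePlayer blackboard bool from the success flag, and only print for damage.
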(event OnPerceptionUpdated(PerceptionComponent)
  (params (UpdatedActors :type Array%20of%20Actor%20Object%20References)))

(fn ConstructionScript)

(fn ManageSight
  (params (Sense :type AI%20Stimulus%20Structure))
  (AI|Components|Blackboard|SetValueasBool (AI|GetBlackboard 0) (Utilities|Name|MakeLiteralName "SeePlayer") (.bsuccessfullysensed Sense)))